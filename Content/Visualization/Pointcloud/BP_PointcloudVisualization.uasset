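; Actor that visualizes a point cloud as collision-free mesh instances on a Hierarchical Instanced Static Mesh.
; The construction script applies mesh, visibility and a dynamic material with color and opacity.
; VisualizePointcloud orients instances along actor-to-point directions, updating them in place when the count matches, otherwise rebuilding.
; A separate hit-result function always rebuilds, using rules for rotation, scale, and placement or omission of misses.
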(event `self.VisualizePointcloud`
  (params (Locations :type "Array of Vector Structure (by ref)"))
  (`self.VisualizeHitsWithLocations` Locations))

(fn `UserConstructionScript`
  ;[1 0.7031 0] Pass the static mesh to the HISM
  (`StaticMeshComponent.SetStaticMesh` (`self.HierarchicalInstancedStaticMesh`) (`self.StaticMesh`))
  ;[0.1484 1 0] Create and pass the material
  (bind _returnvalue (`PrimitiveComponent.CreateDynamicMaterialInstance` (`self.HierarchicalInstancedStaticMesh`) 0 (`self.VisualizationMID`) "None"))
  (`MaterialInstanceDynamic.SetScalarParameterValue` _returnvalue "Opacity" (`self.Opacity`))
  (`MaterialInstanceDynamic.SetVectorParameterValue` _returnvalue "Base Color" (`self.Color`))
  (`PrimitiveComponent.SetMaterial` (`self.HierarchicalInstancedStaticMesh`) 0 _returnvalue)
  ;[1 0.2812 0] disable collision
  (`PrimitiveComponent.SetCollisionEnabled` (`self.HierarchicalInstancedStaticMesh`) "NoCollision")
  ;[0.5703 1 0] Set visibility
  (`SceneComponent.SetVisibility` (`self.HierarchicalInstancedStaticMesh`) (`self.EnableVisualization`) true))

(fn `VisualizeHitsWithHitResults`
  (params (HitResults :type "Array of HitResult Structure"))
  (locals (Local_HitResults :type "Array of HitResult Structure") (Local_CurrentHit :type "HitResult Structure") (Local_CurrentScale :type "Vector Structure" :default (1.0 1.0 1.0)) (Local_CurrentRotation :type "Rotator Structure" :default (struct)) (Local_CurrentLocation :type "Vector Structure" :default (0.0 0.0 0.0)))
  (bind (_bblockinghit _binitialoverlap _time _distance _location _impactpoint _normal _impactnormal _physmat _hitactor _hitcomponent _hitbonename _hititem _elementindex _faceindex _tracestart _traceend) (`GameplayStatics.BreakHitResult` (`local.Local_CurrentHit`)))
  (bind (_bblockinghit_2 _binitialoverlap_2 _time_2 _distance_2 _location_2 _impactpoint_2 _normal_2 _impactnormal_2 _physmat_2 _hitactor_2 _hitcomponent_2 _hitbonename_2 _hititem_2 _elementindex_2 _faceindex_2 _tracestart_2 _traceend_2) (`GameplayStatics.BreakHitResult` (`local.Local_CurrentHit`)))
  (set `local.Local_HitResults` HitResults)
  ;[0 0.8828 1] Clear old instances
  (`InstancedStaticMeshComponent.ClearInstances` (`self.HierarchicalInstancedStaticMesh`))
  (for _array_element (`local.Local_HitResults`)
    (set `local.Local_CurrentHit` _array_element)
    (`|ExecutionSequence`
      (:`then_0`
        ;[1 0.7969 0] Orientation
        (switch `/Sensors/Visualization/Pointcloud/ENUM_OrientationRule` (`self.RotationRule`)
          (:`NewEnumerator0`
            (set `local.Local_CurrentRotation` (`KismetMathLibrary.FindLookAtRotation` _tracestart _traceend)))
          (:`NewEnumerator1`
            (set `local.Local_CurrentRotation` (`KismetMathLibrary.MakeRotFromX` (`.ImpactNormal` (`GameplayStatics.BreakHitResult` (`local.Local_CurrentHit`))))))))
      (:`then_1`
        ;[1 0 0.4219] Scaling
        (switch `/Sensors/Visualization/Pointcloud/ENUM_ScaleRule` (`self.ScaleRule`)
          (:`NewEnumerator0`
            (set `local.Local_CurrentScale` (`self.Scale`)))))
      (:`then_2`
        ;[0.4062 1 0] Manage Location
        (switch `/Sensors/Visualization/Pointcloud/ENUM_LocationRule` (`self.LocationRule`)
          (:`NewEnumerator0`
            (set `local.Local_CurrentLocation` (`.ImpactPoint` (`GameplayStatics.BreakHitResult` (`local.Local_CurrentHit`)))))
          (:`NewEnumerator1`
            (if _bblockinghit_2
              (set `local.Local_CurrentLocation` _impactpoint_2)
              (else
                (set `local.Local_CurrentLocation` _traceend_2))))))
      (:`then_3`
        ;[1 0.5391 0] Only spawn if wanted
        (switch `/Sensors/Visualization/Pointcloud/ENUM_LocationRule` (`self.LocationRule`)
          (:`NewEnumerator0`
            (if (`GameplayStatics.BreakHitResult` (`local.Local_CurrentHit`))
              (`InstancedStaticMeshComponent.AddInstanceWorldSpace` (`self.HierarchicalInstancedStaticMesh`) (`KismetMathLibrary.MakeTransform` (`local.Local_CurrentLocation`) (`local.Local_CurrentRotation`) (`local.Local_CurrentScale`)) :!label _label)))
          (:`NewEnumerator1`
            (goto _label)))))))

(fn `VisualizeHitsWithLocations`
  (params (Locations :type "Array of Vector Structure"))
  (locals (Local_CurrentScale :type "Vector Structure" :default (1.0 1.0 1.0)) (Local_CurrentRotation :type "Rotator Structure" :default (struct)) (Local_CurrentLocation :type "Vector Structure" :default (0.0 0.0 0.0)) (Local_Locations :type "Array of Vector Structure") (Local_SameSize :type Boolean) (Local_ArrayIndex :type Integer))
  (set `local.Local_Locations` Locations)
  ;[0.8516 0 1] Comment
  (set `local.Local_SameSize` (== (`InstancedStaticMeshComponent.GetInstanceCount` (`self.HierarchicalInstancedStaticMesh`)) (`KismetArrayLibrary.Array_Length` (`local.Local_Locations`))))
  (if (not (`local.Local_SameSize`))
    ;[0 0.8828 1] Clear old instances
    (`InstancedStaticMeshComponent.ClearInstances` (`self.HierarchicalInstancedStaticMesh`)))
  (for (_array_element _array_index) (`local.Local_Locations`)
    (set `local.Local_CurrentLocation` _array_element)
    (set `local.Local_ArrayIndex` _array_index)
    (`|ExecutionSequence`
      (:`then_0`
        ;[1 0.7969 0] Orientation
        (set `local.Local_CurrentRotation` (`KismetMathLibrary.FindLookAtRotation` (`self.K2_GetActorLocation`) (`local.Local_CurrentLocation`))))
      (:`then_1`
        ;[1 0 0.4219] Scaling
        (switch `/Sensors/Visualization/Pointcloud/ENUM_ScaleRule` (`self.ScaleRule`)
          (:`NewEnumerator0`
            (set `local.Local_CurrentScale` (`self.Scale`)))))
      (:`then_2`
        (if (`local.Local_SameSize`)
          (`InstancedStaticMeshComponent.UpdateInstanceTransform` (`self.HierarchicalInstancedStaticMesh`) (`local.Local_ArrayIndex`) (`KismetMathLibrary.MakeTransform` (`local.Local_CurrentLocation`) (`local.Local_CurrentRotation`) (`local.Local_CurrentScale`)) true false false)
          (else
            (`InstancedStaticMeshComponent.AddInstanceWorldSpace` (`self.HierarchicalInstancedStaticMesh`) (`KismetMathLibrary.MakeTransform` (`local.Local_CurrentLocation`) (`local.Local_CurrentRotation`) (`local.Local_CurrentScale`)))))))))