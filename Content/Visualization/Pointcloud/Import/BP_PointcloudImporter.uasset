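; BP_PointcloudImporter is an actor that visualizes point cloud data from a DataTable as debug points in the world.
; VisualizePointcloud loops over every row and draws a debug point at the row's coordinates offset by the actor location, with configurable size and duration.
; A toggle colors points either by their stored RGB values or by object ID clamped to 0–255 as grayscale.
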(event `self.ReceiveTick`
  (params (DeltaSeconds :type "Float (single-precision)")))

(fn `UserConstructionScript`)

(fn `VisualizePointcloud`
  (bind _outrownames (`DataTableFunctionLibrary.GetDataTableRowNames` (`self.Pointcloud`)))
  (for _array_element _outrownames
    (bind _returnvalue (`|GetDataTableRow` (`self.Pointcloud`) _array_element)
      (:`then`
        (if (`self.VisualizeObjectID`)
          (bind (_xcoordinate _ycoordinate _zcoordinate _rcolor _gcolor _bcolor _objectid) (break `/Sensors/Visualization/Pointcloud/Import/ST_RGBPointcloud` _returnvalue))
          (bind _returnvalue_2 (`KismetMathLibrary.Clamp` _objectid 0 255))
          ;[1 0.4922 0] Object ID
          (`KismetSystemLibrary.DrawDebugPoint` (+ (`self.K2_GetActorLocation`) (`KismetMathLibrary.MakeVector` _xcoordinate _ycoordinate _zcoordinate)) (`self.Size`) (`KismetMathLibrary.Conv_ColorToLinearColor` (make `Color` (`KismetMathLibrary.Conv_IntToByte` _returnvalue_2) (`KismetMathLibrary.Conv_IntToByte` _returnvalue_2) (`KismetMathLibrary.Conv_IntToByte` _returnvalue_2) 1)) (`self.Duration`))
          (else
            (bind (_xcoordinate_2 _ycoordinate_2 _zcoordinate_2 _rcolor_2 _gcolor_2 _bcolor_2) (break `/Sensors/Visualization/Pointcloud/Import/ST_RGBPointcloud` _returnvalue))
            ;[1 0 0.8672] RGB Color
            (`KismetSystemLibrary.DrawDebugPoint` (+ (`self.K2_GetActorLocation`) (`KismetMathLibrary.MakeVector` _xcoordinate_2 _ycoordinate_2 _zcoordinate_2)) (`self.Size`) (`KismetMathLibrary.Conv_ColorToLinearColor` (make `Color` _bcolor_2 _gcolor_2 _rcolor_2 1)) (`self.Duration`))))))))