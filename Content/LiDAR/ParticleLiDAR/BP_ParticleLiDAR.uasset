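; Particle-based LiDAR sensor actor that produces a point cloud with a Niagara system.
; Construction script feeds channel count, points per laser and vertical/horizontal FOV from the LiDAR parameters into Niagara.
; The actor registers itself as Niagara's export callback, receives particle data and passes it on with its negated location as offset.
; An optional debug mode draws the received points as short-lived debug points.
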(event `self.ReceiveBeginPlay`
  (`NiagaraComponent.SetNiagaraVariableObject` (`self.Niagara`) "User.ExportCallback" self))

(event `self.ReceiveTick`
  (params (DeltaSeconds :type "Float (single-precision)")))

(event `self.ReceiveParticleData`
  (params (Data :type "Array of BasicParticleData Structure (by ref)") (NiagaraSystem :type "NiagaraSystem Object Reference") (SimulationPositionOffset :type "Vector Structure (by ref)"))
  (set `self.ParticleDataArray` Data)
  (`self.PassParticleData` (`self.ParticleDataArray`) (* (`self.K2_GetActorLocation`) -1.0))
  ;[1 1 1] Visualize Points using simple debug points
  (if (`self.EnableDebugVisualization`)
    ;[1 0.2551 0.6607] Example of using the Pointcloud in Blueprint
    (for _array_element (`self.ParticleDataArray`)
      (`KismetSystemLibrary.DrawDebugPoint` (break `BasicParticleData` _array_element) 20.0 (struct :`G` 1.0 :`B` 0.048136 :`A` 1.0) 0.9))))

(fn `UserConstructionScript`
  (bind (_channelcount _pointstoscanwithonelaser _verticalfov _verticalfovoffset _horizontalfov) (break `ParParticleLiDAR` (`self.ParticleLiDARParameters`)))
  ;[1 1 1] Pass the parameters to the particle system
  (`|ExecutionSequence`
    (:`then_0`
      (`NiagaraComponent.SetVariableInt` (`self.Niagara`) "NumChannels" _channelcount))
    (:`then_1`
      (`NiagaraComponent.SetVariableInt` (`self.Niagara`) "ParticlesPerChannel" _pointstoscanwithonelaser))
    (:`then_2`
      (`NiagaraComponent.SetVariableFloat` (`self.Niagara`) "verticalFOV" _verticalfov))
    (:`then_3`
      (`NiagaraComponent.SetVariableFloat` (`self.Niagara`) "HorizontalFOV" _horizontalfov))))